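; Functional test that checks whether every Texture2D under a search path uses the expected texture group (LODGroup).
; It scans the Asset Registry recursively and picks the expected group from the Characters, Environments, Particles or UI folder, with "_N" names selecting normal map groups for the first two.
; Mismatches log CSV-style warnings, fail the test with Error, and are reassigned when EditorOnlyAutoRepair is on.
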(event EventPrepareTest)

(event EventStartTest
  (bind _successed (Private|PrivateTest))
  ;[1 1 1] 終了
  (Class|FunctionalTest|FinishTest (select _successed "Succeeded" "Error") "Texture Path,Now Group,Request Group,"))

(event EventTick
  (params (DeltaSeconds :type Float%20%28single-precision%29)))

(fn ConstructionScript)

(fn PrivateTest
  (bind _returnvalue (Class|AssetRegistryHelpers|GetAssetRegistry))
  (bind _searchpath (Variables|Setting|GetSearchPath))
  (bind (_outassetdata _returnvalue_2) (Class|AssetRegistry|GetAssetsbyPath _returnvalue _searchpath true false))
  (if _returnvalue_2
    (bind _output_get (LocalVariables|SetAssetList _outassetdata))
    (for _array_element _output_get
      (bind _output_get_2 (LocalVariables|SetAssetData _array_element))
      (bind _astexture_2d (Utilities|Casting|CastToTexture2D (Class|AssetRegistryHelpers|GetAsset _output_get_2)))
      (bind _success (Protected|CheckTextureGroup _astexture_2d (LocalVariables|GetAssetData)))
      (if (not _success)
        (LocalVariables|SetRetSuccess false)))
    (return (LocalVariables|GetRetSuccess))
    (else
      ;[1 1 1] 検索パスがおかしい
      (Class|FunctionalTest|AddError "Invalid \"Search Path\"")
      (return false))))

(fn CheckTextureGroup
  (params (Texture :type Texture%202D%20Object%20Reference) (AssetData :type Asset%20Data%20Structure))
  (bind (_packagepath _assetname) (Utilities|Struct|BreakAssetData AssetData))
  ;[1 1 1] 法線マップか
  (LocalVariables|SetIsNormalMap (>= (Utilities|String|FindSubstring (Utilities|String|ToString(Name) (Utilities|Struct|BreakAssetData AssetData)) "_N" true) 0))
  (Utilities|FlowControl|Sequence
    (:then_0
      ;[1 1 1] キャラクター設定
      (if (>= (Utilities|String|FindSubstring (Utilities|String|ToString(Name) (Utilities|Struct|BreakAssetData AssetData)) "/Characters/") 0)
        (LocalVariables|SetRequestGroup (select (LocalVariables|GetIsNormalMap) "TEXTUREGROUP_CharacterNormalMap" "TEXTUREGROUP_Character"))
        (if (Utilities|Enum|Equal(Enum) (Variables|/Script/Engine.Texture|GetLODGroup Texture) (LocalVariables|GetRequestGroup)) :!label _label
          (return true)
          (else
            (Class|FunctionalTest|AddWarning (Utilities|String|ToString(Text) (Utilities|Text|FormatText "{TexturePath}/{TextureName},{NowGroup},{RequestGroup}," (Utilities|Text|ToText(Name) _packagepath) (Utilities|Text|ToText(Name) _assetname) (Utilities|Text|ToText(String) (Utilities|String|EnumtoString (Variables|/Script/Engine.Texture|GetLODGroup Texture))) (Utilities|Text|ToText(String) (Utilities|String|EnumtoString (LocalVariables|GetRequestGroup))))))
            (if (Variables|Setting|Get[EditorOnly]AutoRepair)
              (Variables|/Script/Engine.Texture|SetLODGroup Texture (LocalVariables|GetRequestGroup)))
            (return false)))))
    (:then_1
      ;[1 1 1] 背景設定
      (if (>= (Utilities|String|FindSubstring (Utilities|String|ToString(Name) (Utilities|Struct|BreakAssetData AssetData)) "/Environments/") 0)
        (LocalVariables|SetRequestGroup (select (LocalVariables|GetIsNormalMap) "TEXTUREGROUP_WorldNormalMap" "TEXTUREGROUP_World"))
        (goto _label)))
    (:then_2
      ;[1 1 1] エフェクト設定
      (if (>= (Utilities|String|FindSubstring (Utilities|String|ToString(Name) (Utilities|Struct|BreakAssetData AssetData)) "/Particles/") 0)
        (LocalVariables|SetRequestGroup "TEXTUREGROUP_Effects")
        (goto _label)))
    (:then_3
      ;[1 1 1] UI設定
      (if (>= (Utilities|String|FindSubstring (Utilities|String|ToString(Name) (Utilities|Struct|BreakAssetData AssetData)) "/UI/") 0)
        (LocalVariables|SetRequestGroup "TEXTUREGROUP_UI")
        (goto _label)))
    (:then_4
      ;[0.9074 1 0] テクスチャ設定ない
      (return true))))