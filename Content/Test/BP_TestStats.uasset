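; BP_TestStats is a functional test that exercises stat readback for the Game stat group.
; On test start it waits, enables the group, then waits again so data can accumulate.
; It reads the call count and inclusive and exclusive averages of STAT_TickTime and logs them as one formatted message.
; It always finishes as Succeeded, with no checks on the values.
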(event EventStartTest
  (bind _returnvalue (Utilities|Name|MakeLiteralName "STAT_TickTime"))
  (Utilities|FlowControl|Delay 1.0)
  ;[1 1 1] 有効にしてちょっと待つ
  (Class|AutomationBlueprintFunctionLibrary|EnableStatGroup "Game")
  (Utilities|FlowControl|Delay 1.0)
  ;[1 1 1] 数値を取って表示
  (bind _returnvalue_2 (Class|AutomationBlueprintFunctionLibrary|GetStatCallCount _returnvalue))
  (bind _returnvalue_3 (Class|AutomationBlueprintFunctionLibrary|GetStatIncAverage _returnvalue))
  (bind _returnvalue_4 (Class|AutomationBlueprintFunctionLibrary|GetStatExcAverage _returnvalue))
  (Class|FunctionalTest|LogMessage (Utilities|String|ToString(Text) (Utilities|Text|FormatText "{0} : {1} : {2}" _returnvalue_2 _returnvalue_3 _returnvalue_4)))
  (Class|FunctionalTest|FinishTest "Succeeded"))

(fn ConstructionScript)