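; Functional test that audits a level's actors for performance-related settings and reports offenders as CSV-style warnings.
; StartTest runs PrivateTest over every actor outside the excluded classes and finishes with success or error.
; CheckActor flags enabled actor or component ticks (particles exempt), planar reflection components, and non-static root mobility, except on lights and physics-simulating roots.
; PrivateTest also fails the level when more than one directional light is non-static.
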(event EventPrepareTest)

(event EventStartTest
  (bind _success (Private|PrivateTest))
  ;[1 1 1] 終了
  (Class|FunctionalTest|FinishTest (select _success "Succeeded" "Error") "Actor Name,Tick,Component Tick num,Use Planar Reflection,Mobility no static"))

(event EventTick
  (params (DeltaSeconds :type Float%20%28single-precision%29)))

(fn ConstructionScript)

(fn PrivateTest
  (bind _outactors (Actor|GetAllActorsOfClass "/Script/Engine.Actor"))
  (for _array_element _outactors
    (LocalVariables|SetActor _array_element)
    (LocalVariables|SetActorCheck true)
    ;[1 1 1] チェックしないクラス
    (bind _array_element_2 (Utilities|Array|ForEachLoopwithBreak (LocalVariables|GetExclusionActorClasses) :!label _label)
      (:LoopBody
        (if (or (Utilities|ClassIsChildOf (Utilities|GetClass (LocalVariables|GetActor)) _array_element_2) (== _array_element_2 (Utilities|GetClass (LocalVariables|GetActor))))
          (LocalVariables|SetActorCheck false)
          (goto _label Break)))
      (:Completed
        (if (LocalVariables|GetActorCheck)
          (Utilities|FlowControl|Sequence
            (:then_0
              (bind _success (Private|CheckActor (LocalVariables|GetActor)))
              (if (not _success)
                (LocalVariables|SetRetSuccess false)))
            (:then_1
              (bind _asdirectional_light (Utilities|Casting|CastToDirectionalLight (LocalVariables|GetActor)))
              (if (Utilities|Enum|NotEqual(Enum) (Variables|/Script/Engine.SceneComponent|GetMobility (Variables|/Script/Engine.Actor|GetRootComponent _asdirectional_light)) "Static")
                (Math|Integer|IncrementInt (LocalVariables|GetDirectionalLightNoStatic)))))))))
  (Utilities|FlowControl|Sequence
    (:then_0
      (if (> (LocalVariables|GetDirectionalLightNoStatic) 1)
        (LocalVariables|SetRetSuccess false)
        (Class|FunctionalTest|AddWarning (Utilities|String|ToString(Text) (Utilities|Text|FormatText "Multiple Directional lights that are not static: Num={Num}" (LocalVariables|GetDirectionalLightNoStatic))))))
    (:then_1
      (return (LocalVariables|GetRetSuccess)))))

(fn CheckActor
  (params (Actor :type Actor%20Object%20Reference))
  (bind _rootcomponent (Variables|/Script/Engine.Actor|GetRootComponent Actor))
  (bind _rootcomponent_2 (Variables|/Script/Engine.Actor|GetRootComponent Actor))
  (LocalVariables|SetComponents (Actor|GetComponentsByClass Actor "/Script/Engine.ActorComponent"))
  (Utilities|FlowControl|Sequence
    (:then_0
      ;[1 1 1] パーティクルは走ってもOK
      (Utilities|Casting|CastToEmitter Actor
        (:CastFailed
          (LocalVariables|SetErrorActorTick (Class|Actor|IsActorTickEnabled Actor))
          (for _array_element (LocalVariables|GetComponents)
            (Utilities|Casting|CastToParticleSystemComponent _array_element
              (:CastFailed
                (if (Class|ActorComponent|IsComponentTickEnabled _array_element)
                  (Math|Integer|IncrementInt (LocalVariables|GetComponentTicks)))))))))
    (:then_1
      (for _array_element_2 (LocalVariables|GetComponents)
        (Utilities|Casting|CastToPlanarReflectionComponent _array_element_2)
        (LocalVariables|SetUsePlanarReflection true)))
    (:then_2
      (Utilities|IsValid _rootcomponent
        (:Is%20Valid
          ;[1 1 1] ライトは除外
          (Utilities|Casting|CastToLightComponentBase _rootcomponent
            (:CastFailed
              ;[1 1 1] 物理挙動するなら除外
              (if (not (Class|SceneComponent|IsAnySimulatingPhysics (Variables|/Script/Engine.Actor|GetRootComponent Actor)))
                ;[1 1 1] Static以外はアウト
                (Utilities|IsValid _rootcomponent_2
                  (:Is%20Valid
                    (LocalVariables|SetErrorMobility (Utilities|Enum|NotEqual(Enum) (Variables|/Script/Engine.SceneComponent|GetMobility _rootcomponent_2) "Static"))))))))))
    (:then_3
      (if (Math|Boolean|ORBoolean (LocalVariables|GetErrorActorTick) (> (LocalVariables|GetComponentTicks) 0) (LocalVariables|GetUsePlanarReflection) (LocalVariables|GetErrorMobility))
        (Class|FunctionalTest|AddWarning (Utilities|String|ToString(Text) (Utilities|Text|FormatText "{ActorName},{ActorTick},{ComponentTick},{UsePlanarRef},{Mobility}" (Utilities|Text|ToText(String) (Utilities|GetObjectName Actor)) (Utilities|Text|ToText(Boolean) (LocalVariables|GetErrorActorTick)) (LocalVariables|GetComponentTicks) (Utilities|Text|ToText(Boolean) (LocalVariables|GetUsePlanarReflection)) (Utilities|Text|ToText(Boolean) (LocalVariables|GetErrorMobility)))))
        (return false)
        (else
          (return true))))))