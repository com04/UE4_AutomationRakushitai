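; Functional test that checks project materials against a rule banning Automatically Set Usage in Editor.
; On start it queries the Asset Registry recursively under SearchPath and runs CheckMaterial on assets that cast to Material.
; Each offending material logs a comma-separated warning with its path, name and flag.
; The test finishes as Error if any material fails or the path query fails, otherwise Succeeded.
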(event EventPrepareTest)

(event EventStartTest
  (bind _successed (Private|PrivateTest))
  ;[1 1 1] 終了
  (Class|FunctionalTest|FinishTest (select _successed "Succeeded" "Error") "Texture Path,Auto Usage"))

(event EventTick
  (params (DeltaSeconds :type Float%20%28single-precision%29)))

(fn ConstructionScript)

(fn PrivateTest
  (bind _returnvalue (Class|AssetRegistryHelpers|GetAssetRegistry))
  (bind _searchpath (Variables|Setting|GetSearchPath))
  (bind (_outassetdata _returnvalue_2) (Class|AssetRegistry|GetAssetsbyPath _returnvalue _searchpath true false))
  (if _returnvalue_2
    (bind _output_get (LocalVariables|SetAssetList _outassetdata))
    (for _array_element _output_get
      (bind _output_get_2 (LocalVariables|SetAssetData _array_element))
      (bind _asmaterial (Utilities|Casting|CastToMaterial (Class|AssetRegistryHelpers|GetAsset _output_get_2)))
      (bind _success (Protected|CheckMaterial _asmaterial (LocalVariables|GetAssetData)))
      (if (not _success)
        (LocalVariables|SetRetSuccess false)))
    (return (LocalVariables|GetRetSuccess))
    (else
      ;[1 1 1] 検索パスがおかしい
      (Class|FunctionalTest|AddError "Invalid \"Search Path\"")
      (return false))))

(fn CheckMaterial
  (params (Material :type Material%20Object%20Reference) (AssetData :type Asset%20Data%20Structure))
  (bind (_packagepath _assetname) (Utilities|Struct|BreakAssetData AssetData))
  (if (not (Variables|/Script/Engine.Material|GetbAutomaticallySetUsageInEditor Material))
    (return true)
    (else
      (Class|FunctionalTest|AddWarning (Utilities|String|ToString(Text) (Utilities|Text|FormatText "{MaterialPath}/{MaterialName},{AutoUsage}," (Utilities|Text|ToText(Name) _packagepath) (Utilities|Text|ToText(Name) _assetname) (Utilities|Text|ToText(Boolean) (Variables|/Script/Engine.Material|GetbAutomaticallySetUsageInEditor Material)))))
      (return false))))