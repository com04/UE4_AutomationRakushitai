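; BP_TestLevelJump is a functional test Blueprint that reports level state as test warnings, apparently a temporary probe for level jumps.
; Tick calls OutputInfo, which logs the current level name with its prefix kept, then the display name of every LevelScriptActor in the world.
; PrepareTest and StartTest are empty, and the graph has no assertions or finish call.
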(event EventPrepareTest)

(event EventStartTest)

(event EventTick
  (params (DeltaSeconds :type Float%20%28single-precision%29))
  (CallFunction|OutputInfo))

(fn ConstructionScript)

(fn OutputInfo
  (bind _returnvalue (Game|GetCurrentLevelName false))
  (Class|FunctionalTest|AddWarning (Utilities|String|ToString(Text) (Utilities|Text|FormatText "[{0}]" (Utilities|Text|ToText(String) _returnvalue))))
  (bind _outactors (Actor|GetAllActorsOfClass "/Script/Engine.LevelScriptActor"))
  (for _array_element _outactors
    (Class|FunctionalTest|AddWarning (Utilities|GetDisplayName _array_element))))