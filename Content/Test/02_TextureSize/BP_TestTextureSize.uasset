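; Functional test that flags Texture2D assets whose width or height reaches a maximum size limit.
; PrivateTest uses the Asset Registry to scan the search path recursively, loading each asset and passing textures to CheckTextureSize.
; Each oversized texture logs a comma-separated warning with path and dimensions, matching the header in the finish message.
; Any oversized texture or an invalid search path finishes the test with an Error result.
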(event EventPrepareTest)

(event EventStartTest
  (bind _success (Private|PrivateTest))
  ;[1 1 1] 終了
  (Class|FunctionalTest|FinishTest (select _success "Succeeded" "Error") "Texture Path,Size X,Size Y,"))

(event EventTick
  (params (DeltaSeconds :type Float%20%28single-precision%29)))

(fn ConstructionScript)

(fn PrivateTest
  (bind _returnvalue (Class|AssetRegistryHelpers|GetAssetRegistry))
  (bind _searchpath (Variables|Setting|GetSearchPath))
  (bind (_outassetdata _returnvalue_2) (Class|AssetRegistry|GetAssetsbyPath _returnvalue _searchpath true false))
  (if _returnvalue_2
    (bind _output_get (LocalVariables|SetAssetList _outassetdata))
    (for _array_element _output_get
      (bind _output_get_2 (LocalVariables|SetAssetData _array_element))
      (bind _astexture_2d (Utilities|Casting|CastToTexture2D (Class|AssetRegistryHelpers|GetAsset _output_get_2)))
      (bind _success (Protected|CheckTextureSize _astexture_2d (LocalVariables|GetAssetData)))
      (if (not _success)
        (LocalVariables|SetRetSuccess false)))
    (return (LocalVariables|GetRetSuccess))
    (else
      ;[1 1 1] 検索パスがおかしい
      (Class|FunctionalTest|AddError "Invalid \"Search Path\"")
      (return false))))

(fn CheckTextureSize
  (params (Texture :type Texture%202D%20Object%20Reference) (AssetData :type Asset%20Data%20Structure))
  (bind (_packagepath _assetname) (Utilities|Struct|BreakAssetData AssetData))
  (if (and (< (Class|Texture2D|BlueprintGetSizeX Texture) (Variables|Setting|GetErrorMaxSize)) (< (Class|Texture2D|BlueprintGetSizeY Texture) (Variables|Setting|GetErrorMaxSize)))
    (return true)
    (else
      (Class|FunctionalTest|AddWarning (Utilities|String|ToString(Text) (Utilities|Text|FormatText "{TexturePath}/{TextureName},{SizeX},{SizeY}," (Utilities|Text|ToText(Name) _packagepath) (Utilities|Text|ToText(Name) _assetname) (Class|Texture2D|BlueprintGetSizeX Texture) (Class|Texture2D|BlueprintGetSizeY Texture))))
      (return false))))