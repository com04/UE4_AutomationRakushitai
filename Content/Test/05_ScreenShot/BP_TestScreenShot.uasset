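; Functional test that captures screenshots and a CSV performance profile of the current level for visual and performance checks.
; It sets itself as the view target, then runs a delayed sequence of console commands for base, stat, light complexity and quad overdraw shots, plus a short CsvProfile recording.
; Capture saves shots with UI under a date, hour and level name, also used for the CSV.
; A stationary light overlap step is left disconnected.
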(event EventStartTest
  (bind _returnvalue (Math|DateTime|Now))
  (bind (_year _month _day _hour) (Math|DateTime|BreakDateTime _returnvalue))
  ;[1 1 1] 撮影用のカメラに遷移させる
  (Game|Player|SetViewTargetwithBlend (Game|GetPlayerController 0) self 0.0 "VTBlend_Linear" 0.0 false)
  (Utilities|FlowControl|Delay 0.2)
  ;[1 1 1] 日付からファイル名を
  (bind _returnvalue_2 (Game|GetCurrentLevelName true))
  (Variables|State|SetScreenShotBaseName (Utilities|Text|FormatText "{Year}{Month}{Day}_{Hour}_{Level}" (Utilities|Text|ToText(Integer) _year false false 4) (Utilities|Text|ToText(Integer) _month false false 2) (Utilities|Text|ToText(Integer) _day false false 2) (Utilities|Text|ToText(Integer) _hour false false 2) (Utilities|Text|ToText(String) _returnvalue_2)))
  ;[1 1 1] 普通に撮影
  (Development|ExecuteConsoleCommand "stat none" 0)
  (Utilities|FlowControl|Delay 0.1)
  (Private|Capture "Base")
  (Utilities|FlowControl|Delay 0.1)
  ;[1 1 1] csvprofileを用いたパフォーマンス計測
  (Development|ExecuteConsoleCommand (Utilities|String|ToString(Text) (Utilities|Text|FormatText "CsvProfile Startfile=Profile_{Filename}.csv" (Variables|State|GetScreenShotBaseName))) 0)
  (Development|ExecuteConsoleCommand "CsvProfile Start" 0)
  (Utilities|FlowControl|Delay 2.0)
  (Development|ExecuteConsoleCommand "CsvProfile Stop" 0)
  ;[1 1 1] stat 使って撮影
  (Development|ExecuteConsoleCommand "stat scenerendering" 0)
  (Development|ExecuteConsoleCommand "stat memory" 0)
  (Utilities|FlowControl|Delay 0.5)
  (Private|Capture "Stat")
  (Utilities|FlowControl|Delay 0.1)
  ;[1 1 1] ライト複雑度
  (Development|ExecuteConsoleCommand "stat none" 0)
  (Development|ExecuteConsoleCommand "viewmode LightComplexity" 0)
  (Utilities|FlowControl|Delay 1.0)
  (Private|Capture "LightComplexity")
  (Utilities|FlowControl|Delay 0.1)
  ;[1 1 1] Overdraw
  (Development|ExecuteConsoleCommand "viewmode QuadOverdraw" 0)
  (Utilities|FlowControl|Delay 1.0)
  (Private|Capture "QuadOverdraw")
  (Utilities|FlowControl|Delay 0.1)
  ;[1 1 1] 終了
  (Class|FunctionalTest|FinishTest "Succeeded"))

(fn ConstructionScript)

(fn PrivateTest
  (return false))

(fn Capture
  (params (AddName :type String))
  (Development|ExecuteConsoleCommand (Utilities|String|ToString(Text) (Utilities|Text|FormatText "shot SHOWUI filename={BaseName}_{AddName}" (Variables|State|GetScreenShotBaseName) (Utilities|Text|ToText(String) AddName))) 0))